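; Boingy is a bouncing projectile actor that hops toward the first player's pawn.
; On BeginPlay it turns its yaw to the player and sets a fixed horizontal speed in that direction.
; Each bounce re-aims, scales horizontal velocity by random entries from the Gravities array and also draws gravity scale from that array, making hops erratic.
; Tick caps upward velocity.
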(event OnProjectileBounce(ProjectileMovement)
  (params (ImpactResult :type Hit%20Result%20Structure%20%28by%20ref%29) (ImpactVelocity :type Vector%20%28by%20ref%29 :default "0, 0, 0"))
  (bind _returnvalue (Math|Random|RandomIntegerinRange 0 17))
  (bind _returnvalue_2 (Game|Player|GetPlayerPawn 0))
  (bind _returnvalue_3 (Transformation|GetActorRotation))
  (bind _returnvalue_4 (Transformation|GetActorRotation))
  (bind _returnvalue_5 (Math|Vector|MakeVector 1.0 0.0 0.0))
  (bind _gravities (Variables|Default|GetGravities))
  (bind _projectilemovement (Variables|Default|GetProjectileMovement))
  (bind _returnvalue_6 (Math|Rotator|MakeRotator 0.0 0.0 (.yaw _returnvalue_4)))
  (bind _output (Utilities|Array|Get(acopy) _gravities _returnvalue))
  (bind _returnvalue_7 (Math|Vector|RotateVector _returnvalue_5 _returnvalue_6))
  (bind _returnvalue_8 (* _returnvalue_7 333.333334))
  (Utilities|IsValid _returnvalue_2
    (:Is%20Valid
      (Transformation|SetActorRotation (Math|Rotator|MakeRotator (.roll _returnvalue_3) (.pitch _returnvalue_3) (.yaw (Math|Rotator|FindLookatRotation (Transformation|GetActorLocation) (Transformation|GetActorLocation _returnvalue_2)))))
      (Variables|/Script/Engine.MovementComponent|SetVelocity _projectilemovement (Math|Vector|MakeVector (* _output (.x _returnvalue_8)) (* _output (.y _returnvalue_8)) (.z (Variables|/Script/Engine.MovementComponent|GetVelocity _projectilemovement))))
      (Variables|/Script/Engine.ProjectileMovementComponent|SetProjectileGravityScale (Variables|Default|GetProjectileMovement) _output))))

(event EventBeginPlay
  (bind _returnvalue (Game|Player|GetPlayerPawn 0))
  (bind _returnvalue_2 (Transformation|GetActorRotation))
  (bind _returnvalue_3 (Math|Vector|MakeVector 1.0 0.0 0.0))
  (bind _returnvalue_4 (Transformation|GetActorRotation))
  (bind _projectilemovement (Variables|Default|GetProjectileMovement))
  (bind _returnvalue_5 (Math|Rotator|MakeRotator 0.0 0.0 (.yaw _returnvalue_4)))
  (bind _returnvalue_6 (Math|Vector|RotateVector _returnvalue_3 _returnvalue_5))
  (bind _returnvalue_7 (* _returnvalue_6 333.333334))
  (Utilities|IsValid _returnvalue
    (:Is%20Valid
      (Transformation|SetActorRotation (Math|Rotator|MakeRotator (.roll _returnvalue_2) (.pitch _returnvalue_2) (.yaw (Math|Rotator|FindLookatRotation (Transformation|GetActorLocation) (Transformation|GetActorLocation _returnvalue)))))
      (Variables|/Script/Engine.MovementComponent|SetVelocity _projectilemovement (Math|Vector|MakeVector (.x _returnvalue_7) (.y _returnvalue_7) (.z (Variables|/Script/Engine.MovementComponent|GetVelocity _projectilemovement)))))))

(event Collision|EventActorBeginOverlap
  (params (OtherActor :type Actor%20Object%20Reference)))

(event EventTick
  (params (DeltaSeconds :type Float%20%28single-precision%29))
  (bind _projectilemovement (Variables|Default|GetProjectileMovement))
  (if (> (.z (Variables|/Script/Engine.MovementComponent|GetVelocity _projectilemovement)) 1e+03)
    (Variables|/Script/Engine.MovementComponent|SetVelocity _projectilemovement (Math|Vector|MakeVector (.x (Variables|/Script/Engine.MovementComponent|GetVelocity _projectilemovement)) (.y (Variables|/Script/Engine.MovementComponent|GetVelocity _projectilemovement)) 1e+03))))

(fn ConstructionScript)