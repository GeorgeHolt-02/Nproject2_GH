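; Flying bat enemy that drifts toward the player, then dive-bombs as a suicide attack.
; Tick fakes flapping flight with manual gravity, resetting vertical speed whenever it drops below spawn height, while easing horizontally toward the player.
; Within range it turns to face the player and starts a short timer that enables Dive.
; Diving is a swept straight-line charge; any sphere overlap then spawns BP_Explosion and destroys the bat.
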(event OnComponentBeginOverlap(Sphere)
  (params (OverlappedComponent :type Primitive%20Component%20Object%20Reference) (OtherActor :type Actor%20Object%20Reference) (OtherComp :type Primitive%20Component%20Object%20Reference) (OtherBodyIndex :type Integer) (bFromSweep :type Boolean) (SweepResult :type Hit%20Result%20Structure%20%28by%20ref%29))
  (if (Variables|Default|GetbDive)
    (Game|SpawnActorfromClass "/Game/Blueprints/Mechanics/BP_Explosion.BP_Explosion_C" (Transformation|GetActorTransform) "Undefined" 0 0)
    (Actor|DestroyActor)))

(event EventBeginPlay
  (Variables|Default|SetFallPositionCap (.z (Transformation|GetActorLocation))))

(event Collision|EventActorBeginOverlap
  (params (OtherActor :type Actor%20Object%20Reference)))

(event EventTick
  (params (DeltaSeconds :type Float%20%28single-precision%29))
  (bind _returnvalue (Transformation|GetActorLocation))
  (bind _returnvalue_2 (Game|Player|GetPlayerPawn 0))
  (bind _returnvalue_3 (Transformation|GetActorLocation _returnvalue_2))
  (if (Variables|Default|GetbDive)
    (CallFunction|Crash DeltaSeconds)
    (else
      (Variables|Default|SetFallSpeed (- (Variables|Default|GetFallSpeed) (* (Math|Float|Square (Variables|Default|GetGravity)) DeltaSeconds)))
      (Transformation|SetActorLocation (+ (Transformation|GetActorLocation) (Math|Vector|MakeVector 0.0 0.0 (* (Variables|Default|GetFallSpeed) DeltaSeconds))) false false)
      (if (< (.z (Transformation|GetActorLocation)) (Variables|Default|GetFallPositionCap))
        (CallFunction|FlapUp)
        (if (not (Variables|Default|GetbInCrashMode))
          (if (< (Math|Vector|Distance(Vector) (Transformation|GetActorLocation) (Transformation|GetActorLocation (Game|Player|GetPlayerPawn 0))) 5e+02) :!label _label
            (Transformation|SetActorRotation (Math|Rotator|FindLookatRotation (Transformation|GetActorLocation) (Transformation|GetActorLocation (Game|Player|GetPlayerPawn 0))))
            (Variables|Default|SetbInCrashMode true)
            (if (not (Class|KismetSystemLibrary|TimerExists 0 "Toggle"))
              (Utilities|Time|SetTimerbyFunctionName 0 "Toggle" 1.0))
            (else
              (Transformation|SetActorLocation (+ (Transformation|GetActorLocation) (Math|Vector|MakeVector (/ (- (.x _returnvalue_3) (.x _returnvalue)) 2.5e+02) (/ (- (.y _returnvalue_3) (.y _returnvalue)) 2.5e+02) 0.0)) false false))))
        (else
          (goto _label))))))

(fn ConstructionScript)

(fn FlapUp
  (Variables|Default|SetFallSpeed (Variables|Default|GetFlapForce)))

(fn Toggle
  (Variables|Default|SetbDive true))

(fn Crash
  (params (DeltaT :type Float%20%28double-precision%29))
  (Transformation|SetActorLocation (+ (Transformation|GetActorLocation) (* 5e+02 (Math|Vector|RotateVector "1.000000, 0, 0" (Transformation|GetActorRotation)) DeltaT)) true false))